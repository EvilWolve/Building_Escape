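; Openable door actor that swings open and closed through its OpenDoor component's OnOpen and OnClose events.
; BeginPlay caches the initial rotation, and the DoorSwing timeline adds its OpenAngle as yaw to that rotation each update.
; OnClose plays the same timeline in reverse.
; A Door Sound event track on the timeline plays the Doorlock sound at the door's location.
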(event OnClose(OpenDoor)
  ;[1 1 1] Open door
  (bind _open_angle (Timeline|DoorSwing Reverse)
    (:Update
      (Transformation|SetActorRotation (Math|Rotator|CombineRotators (Variables|Default|GetInitialRotation) (Math|Rotator|MakeRotator 0.0 0.0 _open_angle))))
    (:Door%20Sound
      (Audio|PlaySoundatLocation "/Game/Audio/door-lock.door-lock" (Transformation|GetActorLocation)))))

(event OnOpen(OpenDoor)
  ;[1 1 1] Open door
  (bind _open_angle (Timeline|DoorSwing Play)
    (:Update
      (Transformation|SetActorRotation (Math|Rotator|CombineRotators (Variables|Default|GetInitialRotation) (Math|Rotator|MakeRotator 0.0 0.0 _open_angle))))
    (:Door%20Sound
      (Audio|PlaySoundatLocation "/Game/Audio/door-lock.door-lock" (Transformation|GetActorLocation)))))

(event EventBeginPlay
  ;[1 1 1] Set initial rotation
  (Variables|Default|SetInitialRotation (Transformation|GetActorRotation)))

(fn ConstructionScript)